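; Player Blueprint holding debug experiments in vector math: a beam bounce test and a velocity projection visualizer.
; GetClickLocation takes the cursor hit with Y replaced by the player's, and ShootBeam line-traces to a given point, drawing the hit.
; The bounce test chains both and draws the reflection off the hit normal, but is disconnected from the left-click input.
; VectorProjection draws X velocity projected onto a tilted up vector, but nothing here calls it.
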(event `self.ReceiveTick`
  (params (DeltaSeconds :type "Float (single-precision)")))

(event `EnhancedInput|/Game/Blueprints/Input/Actions/IA_LMB`
  (params (ActionValue :type "Float (double-precision)") (ElapsedSeconds :type "Float (double-precision)") (TriggeredSeconds :type "Float (double-precision)") (InputAction :type "InputAction Object Reference" :default "/Game/Blueprints/Input/Actions/IA_LMB.IA_LMB"))
  ;[0.1844 0.6167 1] Beam Bounce Test
)

(fn `GetClickLocation`
  (returns (ClickLocation :type "Vector Structure"))
  (bind _returnvalue (`KismetMathLibrary.MakeVector` (.x (`.Location` (`GameplayStatics.BreakHitResult` (`PlayerController.GetHitResultUnderCursorByChannel` (`GameplayStatics.GetPlayerController` 0) "TraceTypeQuery1" false)))) (.y (`self.K2_GetActorLocation`)) (.z (`.Location` (`GameplayStatics.BreakHitResult` (`PlayerController.GetHitResultUnderCursorByChannel` (`GameplayStatics.GetPlayerController` 0) "TraceTypeQuery1" false))))))
  (`KismetSystemLibrary.DrawDebugPoint` _returnvalue 5.0 (struct :`R` 1.0 :`A` 1.0) 10.0)
  (return _returnvalue))

(fn `ShootBeam`
  (params (BeamStart :type "Vector Structure") (BeamEnd :type "Vector Structure"))
  (returns (HitResult :type "HitResult Structure") (Beam :type "Vector Structure"))
  (locals (BeamHitResult :type "HitResult Structure") (BeamImpactPoint :type "Vector Structure" :default (0.0 0.0 0.0)))
  (bind _output_get (set `self.StartPoint` BeamStart))
  (bind _outhit (`KismetSystemLibrary.LineTraceSingle` _output_get (`local.BeamEnd`) "TraceTypeQuery1"))
  (bind (_bblockinghit _binitialoverlap _time _distance _location _impactpoint) (`GameplayStatics.BreakHitResult` _outhit))
  (if _bblockinghit
    (`KismetSystemLibrary.DrawDebugLine` (`self.StartPoint`) _impactpoint (struct :`R` 0.372011 :`G` 1.0 :`B` 0.319719 :`A` 1.0) 10.0 1.0)
    (`KismetSystemLibrary.DrawDebugPoint` _impactpoint 5.0 (struct :`R` 1.0 :`G` 1.0 :`A` 1.0) 10.0)
    (return _outhit (- _impactpoint (`self.StartPoint`)))))

(fn `UserConstructionScript`)

(fn `VectorProjection`
  (bind _returnvalue (`self.K2_GetActorLocation`))
  (bind _returnvalue_2 (+ _returnvalue (`KismetMathLibrary.ProjectVectorOnToVector` (`self.Vector_B`) (`self.Vector_aNorm`))))
  (set `self.Vector_aNorm` (+ (`self.GetActorUpVector`) (1.0 0.0 0.0)))
  (set `self.Vector_B` (`KismetMathLibrary.MakeVector` (.x (`self.GetVelocity`))))
  (`KismetSystemLibrary.DrawDebugLine` _returnvalue _returnvalue_2 (struct :`R` 1.0 :`G` 0.827676 :`B` 0.226286 :`A` 1.0) 0.0 2.0)
  (`KismetSystemLibrary.DrawDebugPoint` _returnvalue_2 5.0 (struct :`R` 1.0 :`A` 1.0)))