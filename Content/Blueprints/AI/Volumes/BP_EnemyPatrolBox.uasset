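; BP_EnemyPatrolBox is an AI trigger volume that sets or clears the combat target of its assigned patrol enemies as the player enters or leaves.
; On begin overlap, an actor implementing PlayerInterface is passed to each valid enemy in PatrolEnemies as its combat target.
; On end overlap, those enemies receive an empty combat target.
; RemovePatrolEnemy drops a given enemy from the list.
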(event `self.ReceiveActorBeginOverlap`
  (params (OtherActor :type "Actor Object Reference"))
  (if (`KismetSystemLibrary.DoesImplementInterface` OtherActor "/Script/Omega.PlayerInterface")
    (for _array_element (`self.PatrolEnemies`)
      (`/Engine/EditorBlueprintResources/StandardMacros.IsValid` _array_element
        (:`Is Valid`
          (`EnemyInterface.SetCombatTarget` _array_element OtherActor))))))

(event `self.ReceiveActorEndOverlap`
  (params (OtherActor :type "Actor Object Reference"))
  (if (and (`KismetSystemLibrary.DoesImplementInterface` OtherActor "/Script/Omega.PlayerInterface") (`KismetArrayLibrary.Array_IsNotEmpty` (`self.PatrolEnemies`)))
    (for _array_element (`self.PatrolEnemies`)
      (`/Engine/EditorBlueprintResources/StandardMacros.IsValid` _array_element
        (:`Is Valid`
          (`EnemyInterface.SetCombatTarget` _array_element null))))))

(fn `RemovePatrolEnemy`
  (params (`Enemy to Remove` :type "/Game/Blueprints/Characters/Enemies/BP_Enemy Object Reference"))
  (if (`KismetArrayLibrary.Array_Contains` (`self.PatrolEnemies`) `Enemy to Remove`)
    (`KismetArrayLibrary.Array_RemoveItem` (`self.PatrolEnemies`) `Enemy to Remove`)))

(fn `UserConstructionScript`)