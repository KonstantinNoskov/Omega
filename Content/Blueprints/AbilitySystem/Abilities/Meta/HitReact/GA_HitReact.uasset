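; GA_HitReact is a gameplay ability that plays a hit reaction on an avatar implementing CombatInterface, and otherwise ends immediately.
; It applies GE_HitReact to the owner, then plays the avatar's hit reaction sequence as an animation override on its anim instance.
; It resets the avatar's attack and ends without waiting for the animation, whose completed or cancelled callback is wired to remove the effect.
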(event `self.K2_ActivateAbility`
  (if (`KismetSystemLibrary.DoesImplementInterface` (`self.GetAvatarActorFromActorInfo`) "/Script/Omega.CombatInterface")
    (`|ExecutionSequence`
      (:`then_0`
        (bind _returnvalue (`self.BP_ApplyGameplayEffectToOwner` "/Game/Blueprints/AbilitySystem/GameplayEffects/Meta/GE_HitReact.GE_HitReact_C"))
        (set `self.Active GE_HitReact` _returnvalue))
      (:`then_1`
        (bind _returnvalue_2 (message `CombatInterface.GetHitReactionAnimation` (`self.GetAvatarActorFromActorInfo`)))
        (bind _returnvalue_3 (message `CombatInterface.GetAnimationInstance` (`self.GetAvatarActorFromActorInfo`)))
        (`PaperZDPlaySlotOverrideAction.PlayAnimationOverrideWithCallbacks` _returnvalue_3 _returnvalue_2
          (:`OnCompleted`
            _)
          (:`OnCancelled`
            _))
        (`self.BP_RemoveGameplayEffectFromOwnerWithHandle` (`self.Active GE_HitReact`)))
      (:`then_2`
        (message `CombatInterface.ResetAttack` (`self.GetAvatarActorFromActorInfo`))
        (`self.K2_EndAbility`)))
    (else
      (`self.K2_EndAbility`))))