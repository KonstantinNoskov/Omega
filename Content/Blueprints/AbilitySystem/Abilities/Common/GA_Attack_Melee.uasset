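; Common melee attack Gameplay Ability for avatars implementing CombatInterface.
; It sends AttackMessage to the avatar, then waits for the Combat.Animation.Damage gameplay event.
; On that event, it box-queries living players around the combat socket, excluding the owner, calls CauseDamage on those found and ends the ability.
; A short timer also ends the ability, serving as a fallback.
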(event `self.K2_ActivateAbility`
  (set `self.CharacterOwner` (`self.GetAvatarActorFromActorInfo`))
  (if (`KismetSystemLibrary.DoesImplementInterface` (`self.CharacterOwner`) "/Script/Omega.CombatInterface")
    (`|ExecutionSequence`
      (:`then_0`
        ;[1 0.3944 0.8064] Handle Attack
        (message `CombatInterface.Attack` (`self.CharacterOwner`)))
      (:`then_1`
        (`AbilityTask_WaitGameplayEvent.WaitGameplayEvent` (struct :`TagName` "Combat.Animation.Damage") null
          (:`then`
            (`KismetSystemLibrary.K2_ClearAndInvalidateTimerHandle` (`self.EndAbilityTimer`)))
          (:`EventReceived`
            (bind (_bcombatsocketexist _returnvalue) (message `CombatInterface.GetCombatSocketLocation` (`self.CharacterOwner`)))
            (bind _outoverlappingactors (`OmegaFunctionLibrary.GetAlivePlayersWithinBox` (`self.CharacterOwner`) (`|MakeArray` (`self.CharacterOwner`)) (50.0 10.0 50.0) _returnvalue))
            (if (`KismetArrayLibrary.Array_IsEmpty` _outoverlappingactors)
              (`self.K2_EndAbility` :!label _label)
              (else
                (for _array_element _outoverlappingactors
                  (`self.CauseDamage` _array_element)
                  (goto _label)))))))
      (:`then_2`
        (bind _returnvalue_2 (`KismetSystemLibrary.K2_SetTimerDelegate` (delegate `End Ability Event`) 0.7 false true))
        (set `self.EndAbilityTimer` _returnvalue_2)))))

(event `End Ability Event`
  (`self.K2_EndAbility`))