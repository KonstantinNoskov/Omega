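; Projectile trap prop that grants itself a projectile ability through its Omega ability system and is set up to fire on a looping cooldown timer.
; BeginPlay caches a muzzle location, scaling only the forward vector's X by the offset, which the combat-interface socket getter returns.
; Shoot is currently empty with ability activation disconnected, SpawnTrapProjectile only creates an effect context, and the other combat getters are stubs.
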(event `self.ReceiveBeginPlay`
  (`|ExecutionSequence`
    (:`then_0`
      (`AbilitySystemComponent.K2_GiveAbility` (`self.OmegaAbilitySystem`) (`self.ProjectileAbility`) 1 -1)
      (`self.SetMuzzleLocation`))
    (:`then_1`
      (`KismetSystemLibrary.K2_SetTimerDelegate` (delegate `Shoot`) (`self.FireCooldown`) true))))

(event `Shoot`)

(fn `GetAirAttackAnimations`
  (returns (ReturnValue :type "Array of PaperZDAnimSequence Object Reference"))
  (return))

(fn `GetAnimationInstance`
  (returns (ReturnValue :type "PaperZDAnimInstance Object Reference"))
  (return null))

(fn `GetAttackAnimation`
  (returns (ReturnValue :type "PaperZDAnimSequence Object Reference"))
  (return null))

(fn `GetAttackAnimations`
  (returns (ReturnValue :type "Array of PaperZDAnimSequence Object Reference"))
  (return))

(fn `GetAvatar`
  (returns (ReturnValue :type "Actor Object Reference"))
  (return null))

(fn `GetCombatSocketLocation`
  (returns (bCombatSocketExist :type Boolean) (ReturnValue :type "Vector Structure"))
  (return true (`self.MuzzleLocation`)))

(fn `GetDeathAnimation`
  (returns (ReturnValue :type "PaperZDAnimSequence Object Reference"))
  (return null))

(fn `GetHitReactionAnimation`
  (returns (ReturnValue :type "PaperZDAnimSequence Object Reference"))
  (return null))

(fn `IsAttackWindowOpened`
  (returns (ReturnValue :type Boolean))
  (return false))

(fn `IsComboActivated`
  (returns (ReturnValue :type Boolean))
  (return false))

(fn `IsDead`
  (returns (ReturnValue :type Boolean))
  (return false))

(fn `SetMuzzleLocation`
  (bind (_returnvalue_x _returnvalue_y _returnvalue_z) (`KismetMathLibrary.BreakVector` (`self.GetActorForwardVector`)))
  (set `self.MuzzleLocation` (+ (`self.K2_GetActorLocation`) (`KismetMathLibrary.MakeVector` (* _returnvalue_x (`self.MuzzleOffset`)) _returnvalue_y _returnvalue_z))))

(fn `SpawnTrapProjectile`
  (locals (EffectContextHandle :type "GameplayEffectContextHandle Structure"))
  (set `local.EffectContextHandle` (`AbilitySystemComponent.MakeEffectContext` (`self.OmegaAbilitySystem`))))

(fn `UserConstructionScript`)