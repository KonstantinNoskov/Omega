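; BP_AbilityScroll is an ability scroll actor whose only scripted behavior is a hovering bob.
; Tick adds delta time to a Radians counter, resetting it to zero once it exceeds 360.
; The sine of that counter, scaled by HoverAmplitdude, moves the Box vertically as a per-frame world offset, so travel depends on frame rate.
; No overlap, pickup or ability-granting logic is implemented here.
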(event `self.ReceiveTick`
  (params (DeltaSeconds :type "Float (single-precision)"))
  (bind _output_get (set `self.Radians` (+ DeltaSeconds (`self.Radians`))))
  (if (> _output_get 360.0)
    (set `self.Radians` 0.0))
  (`SceneComponent.K2_AddWorldOffset` (`self.Box`) (`KismetMathLibrary.MakeVector` 0.0 0.0 (* (`KismetMathLibrary.Sin` (`self.Radians`)) (`self.HoverAmplitdude`))) false false))

(fn `UserConstructionScript`)